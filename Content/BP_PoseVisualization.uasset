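; BP_PoseVisualization draws a debug skeleton of joint positions received through an MQTT client.
; Each tick it iterates a bone-to-parent map and looks up both joints in the client's LastJointPositionMap.
; Where both positions exist, it draws a short-lived colored debug line from parent to child, forming the pose.
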(event `self.ReceiveTick`
  (params (DeltaSeconds :type "Float (single-precision)"))
  (bind _lastjointpositionmap (`/Pose2Twin/BP_MQTTClient.LastJointPositionMap` (`self.BP_MQTTClient`)))
  (`/Engine/EditorBlueprintResources/StandardMacros.IsValid` (`self.BP_MQTTClient`)
    (:`Is Valid`
      (bind _keys (`BlueprintMapLibrary.Map_Keys` (`self.BoneParentMap`)))
      (for _array_element _keys
        (bind (_value _returnvalue) (`BlueprintMapLibrary.Map_Find` _lastjointpositionmap (`BlueprintMapLibrary.Map_Find` (`self.BoneParentMap`) _array_element)))
        (bind (_value_2 _returnvalue_2) (`BlueprintMapLibrary.Map_Find` _lastjointpositionmap _array_element))
        (if (and _returnvalue _returnvalue_2)
          (`KismetSystemLibrary.DrawDebugLine` _value _value_2 (struct :`R` 0.870417 :`B` 1.0 :`A` 1.0) 0.1 2.0))))))

(fn `UserConstructionScript`)