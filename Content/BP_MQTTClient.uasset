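; BP_MQTTClient streams pose joint positions from a pose2twin service over MQTT and visualizes them as short-lived debug points.
; On connect it publishes a subscribe request declaring Unreal's axis convention and unit scale, then listens on the stream topic.
; JointsFromJSON turns each message into a name-to-vector map whose values are drawn.
; EndPlay publishes an unsubscribe request for the stream.
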(event `self.ReceiveBeginPlay`
  (bind _returnvalue (`MqttUtilitiesBPL.CreateMqttClient` (`self.MQTTConfig`)))
  (bind _output_get (set `self.MQTTClient` _returnvalue))
  (`MqttClientInterface.Connect` :`self` _output_get :`onConnectCallback` (delegate `OnConnect`))
  (`MqttClientInterface.SetOnMessageHandler` (`self.MQTTClient`) (delegate `OnMQTTMessage`)))

(event `OnMQTTMessage`
  (params (message :type "MqttMessage Structure"))
  (bind _outjsonobject (`JsonBlueprintFunctionLibrary.FromString` message_Message))
  (bind _values (`BlueprintMapLibrary.Map_Values` (`self.JointsFromJSON` _outjsonobject)))
  (for _array_element _values
    (`KismetSystemLibrary.DrawDebugPoint` _array_element 15.0 (struct :`R` 0.639882 :`B` 1.0 :`A` 1.0) 0.2)))

(event `OnConnect`
  (`MqttClientInterface.Publish` (`self.MQTTClient`) (make `MqttMessage` "{\"topic_id\": \"unreal\", \"forward\": [1, 0, 0], \"up\": [0, 0, 1], \"right\": [0, 1, 0], \"unit_scale\": 100}" "pose2twin/subscribe"))
  (`MqttClientInterface.Subscribe` (`self.MQTTClient`) "pose2twin/stream/unreal" 0))

(event `self.ReceiveEndPlay`
  (params (EndPlayReason :type "EEndPlayReason Enum" :default "Destroyed"))
  (`MqttClientInterface.Publish` (`self.MQTTClient`) (make `MqttMessage` "{\"topic_id\": \"unreal\"}" "pose2twin/unsubscribe")))

(fn `JointsFromJSON`
  (params (JsonObject :type "JsonObjectWrapper Structure (by ref)"))
  (returns (JointPositionMap :type "Map of String to Vector Structure"))
  (locals (Result :type "Map of String to Vector Structure"))
  (bind _fieldnames (`JsonBlueprintFunctionLibrary.GetFieldNames` JsonObject))
  (for _array_element _fieldnames
    (bind _outvalue (`|GetJsonField` JsonObject _array_element))
    (`BlueprintMapLibrary.Map_Add` (`local.Result`) _array_element (`KismetMathLibrary.MakeVector` (`|GetArrayItem` _outvalue) (`|GetArrayItem` _outvalue 1) (`|GetArrayItem` _outvalue 2))))
  (return (`local.Result`)))

(fn `UserConstructionScript`)